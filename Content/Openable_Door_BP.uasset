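; Door actor that swings open and closed in response to open and close requests from OpenDoor.
; On BeginPlay it stores its starting rotation as the reference for the swing.
; The DoorSmoothRot timeline adds an animated yaw to that rotation, playing to open and reversing to close.
; An event track on the same timeline plays the door sound at the actor's location.
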(event OnOpenRequest(OpenDoor)
  (bind _doorangle (Timeline|DoorSmoothRot Play)
    (:Update
      (Transformation|SetActorRotation (Math|Rotator|CombineRotators (Math|Rotator|MakeRotator 0.0 0.0 _doorangle) (Variables|Default|GetDoorInitialRotation))))
    (:SoundTrack
      (Audio|PlaySoundatLocation "/Game/Audio/open_door_1.open_door_1" (Transformation|GetActorLocation) "0, 0, 0" 1.0 1.0 0.0 0 0 0))))

(event OnCloseRequest(OpenDoor)
  (bind _doorangle (Timeline|DoorSmoothRot Reverse)
    (:Update
      (Transformation|SetActorRotation (Math|Rotator|CombineRotators (Math|Rotator|MakeRotator 0.0 0.0 _doorangle) (Variables|Default|GetDoorInitialRotation))))
    (:SoundTrack
      (Audio|PlaySoundatLocation "/Game/Audio/open_door_1.open_door_1" (Transformation|GetActorLocation) "0, 0, 0" 1.0 1.0 0.0 0 0 0))))

(event EventBeginPlay
  (Variables|Default|SetDoorInitialRotation (Transformation|GetActorRotation)))

(fn ConstructionScript)